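; Drivable Chaos vehicle with an orbit camera, speedometer HUD and timed checkpoint race.
; An overlap box offers the car to BP_FirstPersonCharacter; F spawns and possesses a new character at the exit point.
; Tick drives engine audio and per-wheel effects: landing impacts, skid sound and surface-dependent Niagara smoke.
; Start checkpoints begin the timer; finish counts only after all intermediate checkpoints are collected, destroying each as it registers.
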(event `self.ReceiveBeginPlay`
  (`|ExecutionSequence`
    (:`then_0`
      (bind _returnvalue (`|CreateWidget` "/Game/NewVehicle/Speedmeter_w.Speedmeter_w_C"))
      (bind _output_get (set `self.HUD` _returnvalue))
      (`UserWidget.AddToViewport` _output_get 0)
      (`AudioComponent.Stop` (`self.engine_sound_Cue`))
      (`ActorComponent.K2_DestroyComponent` (`self.VehicleMovementComponent`))
      (`KismetSystemLibrary.Delay` 0.5)
      (`self.SetActorTickEnabled` true))
    (:`then_1`
      (set `self.ParticleEmitters` (`|MakeArray` (`self.Niagara_FL`) (`self.Niagara_FR`) (`self.Niagara_BL`) (`self.Niagara_BR`))))
    (:`then_2`
      ;[1 1 1] Get all checkpoints in the level
      (bind _outactors (`GameplayStatics.GetAllActorsOfClass` "/Game/NewVehicle/BP_Checkpoint.BP_Checkpoint_C"))
      (for _array_element _outactors
        (if (`/Game/NewVehicle/BP_Checkpoint.IsCheckpoint` _array_element)
          (`KismetArrayLibrary.Array_AddUnique` (`self.CheckpointProgress`) _array_element))))))

(event `InputAction|Handbrake` :paused true
  (params (Key :type "Key Structure"))
  (bind _chaoswheeledvehiclemovement (`self.ChaosWheeledVehicleMovement`))
  (:`Pressed`
    (set `self.Handbrake?` true)
    (`ChaosVehicleMovementComponent.SetHandbrakeInput` _chaoswheeledvehiclemovement true))
  (:`Released`
    (set `self.Handbrake?` false)
    (`ChaosVehicleMovementComponent.SetHandbrakeInput` _chaoswheeledvehiclemovement false)))

(event `InputAxis|MoveForward` :paused true
  (params (AxisValue :type "Float (single-precision)"))
  (`ChaosVehicleMovementComponent.SetThrottleInput` (`self.ChaosWheeledVehicleMovement`) AxisValue))

(event `InputAxis|MoveRight` :paused true
  (params (AxisValue :type "Float (single-precision)"))
  (`ChaosVehicleMovementComponent.SetSteeringInput` (`self.ChaosWheeledVehicleMovement`) AxisValue))

(event `InputAxis|Brake`
  (params (AxisValue :type "Float (single-precision)"))
  (`ChaosVehicleMovementComponent.SetBrakeInput` (`self.ChaosWheeledVehicleMovement`) AxisValue)
  (if (or (> AxisValue 0.0) (`self.Handbrake?`))
    (`MaterialInstanceDynamic.SetVectorParameterValue` (`self.ChassisMat`) "BrakeLightColor" (make `LinearColor` 20.0))
    (else
      (`MaterialInstanceDynamic.SetVectorParameterValue` (`self.ChassisMat`) "BrakeLightColor" (make `LinearColor` 0.467784 0.0 0.0 1.0)))))

(event `InputAxisKey|MouseX`
  (params (AxisValue :type "Float (single-precision)"))
  (`SceneComponent.K2_AddRelativeRotation` (`self.SpringArm`) (`KismetMathLibrary.MakeRotator` 0.0 0.0 AxisValue) false false))

(event `InputAxisKey|MouseY`
  (params (AxisValue :type "Float (single-precision)"))
  (`SceneComponent.K2_AddRelativeRotation` (`self.SpringArm`) (`KismetMathLibrary.MakeRotator` 0.0 AxisValue) false false))

(event `self.ReceiveTick`
  (params (DeltaSeconds :type "Float (single-precision)"))
  (`AudioComponent.SetFloatParameter` (`self.engine_sound_Cue`) "RPM" (`ChaosVehicleMovementComponent.GetForwardSpeed` (`self.ChaosWheeledVehicleMovement`)))
  (`self.CarEffects`)
  (if (`self.IsRaceActive`)
    (`/Game/NewVehicle/Speedmeter_w.UpdateLapTimer` (`self.HUD`) (`KismetMathLibrary.FromSeconds` (- (`KismetSystemLibrary.GetGameTimeInSeconds`) (`self.StartTime`))))))

(event `self.Box.OnComponentBeginOverlap`
  (params (OverlappedComponent :type "PrimitiveComponent Object Reference") (OtherActor :type "Actor Object Reference") (OtherComp :type "PrimitiveComponent Object Reference") (OtherBodyIndex :type Integer) (bFromSweep :type Boolean) (SweepResult :type "HitResult Structure (by ref)"))
  (bind _asbp_first_person_character (cast `/Game/FirstPerson/Blueprints/BP_FirstPersonCharacter` OtherActor))
  (set `/Game/FirstPerson/Blueprints/BP_FirstPersonCharacter.CarAvailable?` true _asbp_first_person_character)
  (set `/Game/FirstPerson/Blueprints/BP_FirstPersonCharacter.AvailableCarRef` self _asbp_first_person_character))

(event `self.Box.OnComponentEndOverlap`
  (params (OverlappedComponent :type "PrimitiveComponent Object Reference") (OtherActor :type "Actor Object Reference") (OtherComp :type "PrimitiveComponent Object Reference") (OtherBodyIndex :type Integer))
  (bind _asbp_first_person_character (cast `/Game/FirstPerson/Blueprints/BP_FirstPersonCharacter` OtherActor))
  (set `/Game/FirstPerson/Blueprints/BP_FirstPersonCharacter.CarAvailable?` false _asbp_first_person_character)
  (set `/Game/FirstPerson/Blueprints/BP_FirstPersonCharacter.AvailableCarRef` null _asbp_first_person_character))

(event `Key|F`
  (params (Key :type "Key Structure"))
  (:`Pressed`
    (bind _returnvalue (`|SpawnActorFromClass` "/Game/FirstPerson/Blueprints/BP_FirstPersonCharacter.BP_FirstPersonCharacter_C" (`SceneComponent.K2_GetComponentToWorld` (`self.CarExitLocation`)) "Undefined" "OverrideRootScale" null null))
    (`Controller.Possess` (`GameplayStatics.GetPlayerController` 0) _returnvalue)))

(event `self.ReceivePossessed`
  (params (NewController :type "Controller Object Reference"))
  (`AudioComponent.Play` (`self.engine_sound_Cue`) 1.0))

(event `self.ReceiveUnpossessed`
  (params (OldController :type "Controller Object Reference"))
  (`AudioComponent.StopDelayed` (`self.engine_sound_Cue`) 0.5))

(event `self.Box1.OnComponentBeginOverlap`
  (params (OverlappedComponent :type "PrimitiveComponent Object Reference") (OtherActor :type "Actor Object Reference") (OtherComp :type "PrimitiveComponent Object Reference") (OtherBodyIndex :type Integer) (bFromSweep :type Boolean) (SweepResult :type "HitResult Structure (by ref)"))
  (`self.ProgressCheckpoint` OtherActor))

(fn `CarEffects`
  (bind _chaoswheeledvehiclemovement (`self.ChaosWheeledVehicleMovement`))
  (bind _skiddingsound (`self.SkiddingSound`))
  (set `self.SkidVolume` 0.0)
  (set `self.AnyTireSkidding?` false)
  (for _index (range (`ChaosWheeledVehicleMovementComponent.GetNumWheels` _chaoswheeledvehiclemovement))
    (`|ExecutionSequence`
      (:`then_0`
        (bind (_bincontact _contactpoint _physmaterial _normalizedsuspensionlength _springforce _slipangle _bisslipping _slipmagnitude _bisskidding _skidmagnitude) (`ChaosWheeledVehicleMovementComponent.BreakWheelStatus` (`ChaosWheeledVehicleMovementComponent.GetWheelState` _chaoswheeledvehiclemovement _index)))
        ;[1 1 1] Car Impact Landing
        (if (> _springforce 3100000.0)
          (`GameplayStatics.PlaySoundAtLocation` "/Game/Audio/SoundWaves/Vehicle/Impacts/VehToVeh/Metal_Roof/sfx_Veh_Impact_Roof_nl_02.sfx_Veh_Impact_Roof_nl_02" _contactpoint (struct) 0.6 1.4 0.0 null null null null)))
      (:`then_1`
        ;[1 1 1] Check if any tire is skidding
        (if _bisskidding
          (set `self.AnyTireSkidding?` true)
          (set `self.SkidVolume` (+ (`self.SkidVolume`) (`KismetMathLibrary.FClamp` (`KismetMathLibrary.NormalizeToRange` (`KismetMathLibrary.Abs` _skidmagnitude) 0.0 100.0) 0.0 1.2)))))
      (:`then_2`
        ;[0.4336 1 0.4546] Change niagara particle type depending on the surface
        (if (and _bincontact (or _bisskidding _bisslipping))
          (bind _output (`|GetArrayItem` (`self.ParticleEmitters`) _index))
          (`ActorComponent.SetActive` _output true false)
          (switch `EPhysicalSurface` (`PhysicalMaterial.SurfaceType` _physmaterial)
            (:`SurfaceType1`
              (`NiagaraComponent.SetAsset` _output "/Game/Realistic_Starter_VFX_Pack_Vol2/Particles/Smoke/P_Smoke_B_road.P_Smoke_B_road" false))
            (:`SurfaceType9`
              (`NiagaraComponent.SetAsset` _output "/Game/Realistic_Starter_VFX_Pack_Vol2/Particles/Smoke/P_Smoke_B_Dirt.P_Smoke_B_Dirt" false)))
          (else
            (`ActorComponent.Deactivate` (`|GetArrayItem` (`self.ParticleEmitters`) _index)))))))
  ;[1 0.7805 0.7706] Start/Stop Sound - Skidding
  (if (`self.AnyTireSkidding?`)
    (`/Engine/EditorBlueprintResources/StandardMacros.IsValid` _skiddingsound
      (:`Is Valid`
        (if (not (`AudioComponent.IsPlaying` _skiddingsound))
          (bind _returnvalue (`GameplayStatics.SpawnSoundAttached` "/Game/Audio/SoundWaves/Ambient/Veh/Skids/sfx_LeaveBehind_amb_Swt_Skid_nl_01.sfx_LeaveBehind_amb_Swt_Skid_nl_01" (`self.Mesh`) "None" (0.0 0.0 0.0) (struct) "KeepRelativeOffset" false (`self.SkidVolume`) 1.0 0.0 null null false :!label _label))
          (set `self.SkiddingSound` _returnvalue)))
      (:`Is Not Valid`
        (goto _label)))
    (else
      (`/Engine/EditorBlueprintResources/StandardMacros.IsValid` (`self.SkiddingSound`)
        (:`Is Valid`
          (`AudioComponent.Stop` (`self.SkiddingSound`)))))))

(fn `ProgressCheckpoint`
  (params (Object :type "Object Object Reference"))
  (locals (ActiveCheckpoint :type "/Game/NewVehicle/BP_Checkpoint Object Reference"))
  (bind _activecheckpoint (`local.ActiveCheckpoint`))
  (bind _activecheckpoint_2 (`local.ActiveCheckpoint`))
  (bind _asbp_checkpoint (cast `/Game/NewVehicle/BP_Checkpoint` Object))
  (set `local.ActiveCheckpoint` _asbp_checkpoint)
  (if (`/Game/NewVehicle/BP_Checkpoint.IsStart` _asbp_checkpoint)
    (set `self.StartTime` (`KismetSystemLibrary.GetGameTimeInSeconds`))
    (set `self.IsRaceActive` true)
    (`self.K2_DestroyActor` (`local.ActiveCheckpoint`))
    (elif (`/Game/NewVehicle/BP_Checkpoint.IsFinish` _asbp_checkpoint)
      (if (== (`KismetArrayLibrary.Array_Length` (`self.CheckpointProgress`)) 0)
        (set `self.FinishTime` (- (`KismetSystemLibrary.GetGameTimeInSeconds`) (`self.StartTime`)))
        (`/Game/NewVehicle/Speedmeter_w.SendLapComplete` (`self.HUD`))
        (set `self.IsRaceActive` false)
        (`self.K2_DestroyActor` (`local.ActiveCheckpoint`)))
      (elif (and (`/Game/NewVehicle/BP_Checkpoint.IsCheckpoint` _activecheckpoint) (`KismetArrayLibrary.Array_Contains` (`self.CheckpointProgress`) _activecheckpoint))
        (`KismetArrayLibrary.Array_RemoveItem` (`self.CheckpointProgress`) _activecheckpoint_2)
        (`self.K2_DestroyActor` _activecheckpoint_2)
        (`/Game/NewVehicle/Speedmeter_w.OnCheckpoint` (`self.HUD`))))))

(fn `UserConstructionScript`
  (bind _returnvalue (`PrimitiveComponent.CreateDynamicMaterialInstance` (`self.Mesh`) 0 "/Game/Vehicles/SportsCar/Materials/MI_SportsCar_Chassis.MI_SportsCar_Chassis" "None"))
  (set `self.ChassisMat` _returnvalue))